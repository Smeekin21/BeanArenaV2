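; DeathZone_BP is a kill volume that zeroes the health of any BP_MechanicPlayerCharacter entering its Box.
; BeginPlay casts and caches local players 0 and 1 as Player1 and Player2.
; On overlap it prints a debug string, sets CurrentHealth to zero, then calls the character's Damage with Player1 always as Target.
; Player2 is never read, and a note flags unfinished team colour handling.
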(event `self.ReceiveBeginPlay`
  (bind _asbp_mechanic_player_character (cast `/Game/ThirdPerson/Blueprints/BP_MechanicPlayerCharacter` (`GameplayStatics.GetPlayerCharacter` 0)))
  (set `self.Player 1` _asbp_mechanic_player_character)
  (bind _asbp_mechanic_player_character_2 (cast `/Game/ThirdPerson/Blueprints/BP_MechanicPlayerCharacter` (`GameplayStatics.GetPlayerCharacter` 1)))
  (set `self.Player 2` _asbp_mechanic_player_character_2))

(event `self.Box.OnComponentBeginOverlap`
  (params (OverlappedComponent :type "PrimitiveComponent Object Reference") (OtherActor :type "Actor Object Reference") (OtherComp :type "PrimitiveComponent Object Reference") (OtherBodyIndex :type Integer) (bFromSweep :type Boolean) (SweepResult :type "HitResult Structure (by ref)"))
  ; DaethZone (Need colour to change to same tesam
  (`KismetSystemLibrary.PrintString` "Hello")
  (bind _asbp_mechanic_player_character (cast `/Game/ThirdPerson/Blueprints/BP_MechanicPlayerCharacter` OtherActor))
  (set `/Game/ThirdPerson/Blueprints/BP_MechanicPlayerCharacter.Current Health` 0.0 _asbp_mechanic_player_character)
  (`/Game/ThirdPerson/Blueprints/BP_MechanicPlayerCharacter.Damage` _asbp_mechanic_player_character 100.0 0.0 false (`self.Player 1`)))

(fn `UserConstructionScript`)