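; Automatic gun weapon that fires randomly colored jelly bean projectiles for the mechanic player character.
; While fire is held, a looping timer at the fire rate calls Fire.
; Fire spawns a projectile at the character weapon's barrel socket, aimed along the follow camera with an upward arc offset, and spends ammo.
; An empty magazine stops firing and triggers a delayed automatic refill.
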(event `Reload`
  (if (<= (`self.AmmoAmount`) 0)
    (`KismetSystemLibrary.PrintString` "Is Reloading")
    (`KismetSystemLibrary.Delay` 5.0)
    (set `self.AmmoAmount` (`self.MaxAmmoAmount`))
    (set `self.HasAmmo?` true)
    (`KismetSystemLibrary.PrintString` "Ready")))

(event `FireStarted`
  (if (`self.HasAmmo?`)
    (set `self.Firing` true)
    (`self.FireEvent`)
    (bind _returnvalue (`KismetSystemLibrary.K2_SetTimerDelegate` (delegate `FireEvent`) (`self.Fire Rate`) true))
    (set `self.Timer` _returnvalue)))

(event `FireEvent`
  (if (`self.Firing`)
    (`KismetSystemLibrary.PrintString` "ahhhhh")
    (`self.Fire`)))

(event `FireCompleted`
  (`self.Stop Fire`))

(event `Stop Fire`
  (set `self.Firing` false)
  (`KismetSystemLibrary.K2_ClearAndInvalidateTimerHandle` (`self.Timer`)))

(fn `Fire`
  (bind _asbp_mechanic_player_character (cast `/Game/ThirdPerson/Blueprints/BP_MechanicPlayerCharacter` (`GameplayStatics.GetPlayerCharacter` 0)))
  (bind _returnvalue_location (`KismetMathLibrary.BreakTransform` (`SceneComponent.GetSocketTransform` (`/Game/ThirdPerson/Blueprints/BP_MechanicPlayerCharacter.Weapon` _asbp_mechanic_player_character) "Barrel_Start" "RTS_World")))
  (bind (_returnvalue_roll _returnvalue_pitch _returnvalue_yaw) (`KismetMathLibrary.BreakRotator` (`KismetMathLibrary.Conv_VectorToRotator` (`SceneComponent.GetForwardVector` (`/Game/ThirdPerson/Blueprints/BP_MechanicPlayerCharacter.FollowCamera` _asbp_mechanic_player_character)))))
  (bind _returnvalue (`|SpawnActorFromClass` "/Game/Blueprints/BP_JellyBean_Projectile.BP_JellyBean_Projectile_C" (`KismetMathLibrary.MakeTransform` (+ (`SceneComponent.GetForwardVector` (`/Game/ThirdPerson/Blueprints/BP_MechanicPlayerCharacter.FollowCamera` _asbp_mechanic_player_character)) _returnvalue_location) (`KismetMathLibrary.MakeRotator` _returnvalue_roll (+ _returnvalue_pitch (`self.Arc amount`)) _returnvalue_yaw)) "Undefined" "MultiplyWithRoot" null self null))
  (`PrimitiveComponent.SetMaterial` (`/Game/Blueprints/BP_JellyBean_Projectile.Sphere` _returnvalue) 0 (`KismetArrayLibrary.Array_Random` (`self.Material Array`)))
  (set `self.AmmoAmount` (- (`self.AmmoAmount`) 1))
  (if (<= (`self.AmmoAmount`) 0)
    (set `self.Firing` false)
    (set `self.HasAmmo?` false)
    (`self.Reload`)))

(fn `UserConstructionScript`)