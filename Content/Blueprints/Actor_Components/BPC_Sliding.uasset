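; BPC_Sliding is an actor component that gives the player character a slide with cooldown and looping dust effects.
; StartSlide requests crouch, launches the owner forward, lowers friction and braking, and ignores move input.
; Tick adds downhill force from a double cross product of the floor normal, caps speed, and calls EndSlide when slow.
; EndSlide restores movement and input, using upward traces to decide when to uncrouch.
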(event `self.ReceiveBeginPlay`
  (bind _returnvalue (`Actor.GetComponentByClass` (`self.GetOwner`) "/Script/Engine.CharacterMovementComponent"))
  ; Begin Play
  (`/Engine/EditorBlueprintResources/StandardMacros.IsValid` _returnvalue
    (:`Is Valid`
      (set `self.CharacterMovement` _returnvalue)
      (set `self.Ground Friction` (`CharacterMovementComponent.GroundFriction` (`self.CharacterMovement`)))
      (set `self.Braking Deceleration Walking` (`CharacterMovementComponent.BrakingDecelerationWalking` (`self.CharacterMovement`)))
      (set `self.Gravity Scale` (`CharacterMovementComponent.GravityScale` (`self.CharacterMovement`)))
      (bind _asbp_mechanic_player_character (cast `/Game/ThirdPerson/Blueprints/BP_MechanicPlayerCharacter` (`GameplayStatics.GetPlayerCharacter` 0)))
      (set `self.As BP Mechanic Player Character` _asbp_mechanic_player_character))))

(event `Key|Gamepad_DPad_Up`
  (params (Key :type "Key Structure")))

(event `Key|One`
  (params (Key :type "Key Structure")))

(event `StartSlide`
  (bind _returnvalue (`Actor.GetActorUpVector` (`self.GetOwner`)))
  (bind (_currentfloor_bblockinghit _currentfloor_bwalkablefloor _currentfloor_blinetrace _currentfloor_floordist _currentfloor_linedist _currentfloor_hitresult) (break `FindFloorResult` (`CharacterMovementComponent.CurrentFloor` (`self.CharacterMovement`))))
  ; StartSlide
  (if (not (`self.SlideCooldown`))
    (set `self.SlideCooldown` true)
    (`self.OnStartStopCrouch` true)
    (set `MovementComponent.Velocity` (* (`Actor.GetActorForwardVector` (`self.GetOwner`)) 1000.0) (`self.CharacterMovement`))
    (set `CharacterMovementComponent.GroundFriction` 0.0 (`self.CharacterMovement`))
    (set `CharacterMovementComponent.BrakingDecelerationWalking` 500.0 (`self.CharacterMovement`))
    (bind _output_get (set `self.Floor Angle` (`.Normal` (`GameplayStatics.BreakHitResult` _currentfloor_hitresult))))
    (if (not (== _output_get _returnvalue :`ErrorTolerance` 0.1))
      (`CharacterMovementComponent.AddForce` (`self.CharacterMovement`) (* (`KismetMathLibrary.Cross_VectorVector` _output_get (`KismetMathLibrary.Cross_VectorVector` _output_get _returnvalue)) 500000.0)))
    (`Controller.SetIgnoreMoveInput` (`GameplayStatics.GetPlayerController` 0) true)
    (`self.SetComponentTickEnabled` true)
    (set `self.Sliding` true)
    (bind _returnvalue_2 (`KismetSystemLibrary.K2_SetTimerDelegate` (delegate `DustEffect`) 0.1 true))
    (set `self.DustTimer` _returnvalue_2)))

(event `DustEffect`
  (bind _returnvalue (`NiagaraFunctionLibrary.SpawnSystemAtLocation` "/Game/VFX/Confetti_Celebration/Slide_Dust/NS_SlideDust.NS_SlideDust" (`Actor.K2_GetActorLocation` (`self.GetOwner`)))))

(event `self.ReceiveTick`
  (params (DeltaSeconds :type "Float (single-precision)"))
  (bind _returnvalue (`Actor.GetVelocity` (`self.GetOwner`)))
  (bind (_currentfloor_bblockinghit _currentfloor_bwalkablefloor _currentfloor_blinetrace _currentfloor_floordist _currentfloor_linedist _currentfloor_hitresult) (break `FindFloorResult` (`CharacterMovementComponent.CurrentFloor` (`self.CharacterMovement`))))
  ; Event Tick
  (`CharacterMovementComponent.AddForce` (`self.CharacterMovement`) (`self.Check if floor is sloped` (`.Normal` (`GameplayStatics.BreakHitResult` _currentfloor_hitresult))))
  (`|ExecutionSequence`
    (:`then_0`
      (if (> (`KismetMathLibrary.VSize` _returnvalue) 1000.0)
        (set `MovementComponent.Velocity` (* (`KismetMathLibrary.Normal` _returnvalue) 1000.0) (`self.CharacterMovement`))))
    (:`then_1`
      (if (< (`KismetMathLibrary.VSize` (`Actor.GetVelocity` (`self.GetOwner`))) 300.0)
        (`self.EndSlide`)))))

(event `EndSlide`
  (bind _charactermovement (`self.CharacterMovement`))
  (bind _returnvalue (`Actor.K2_GetActorLocation` (`self.GetOwner`)))
  ; EndSlide
  (`KismetSystemLibrary.K2_ClearAndInvalidateTimerHandle` (`self.DustTimer`))
  (`/Engine/EditorBlueprintResources/StandardMacros.IsValid` (stale `DustEffect` _returnvalue)
    (:`Is Valid`
      (`self.K2_DestroyComponent` (stale `DustEffect` _returnvalue))
      (set `CharacterMovementComponent.GroundFriction` (`self.Ground Friction`) _charactermovement)
      (set `CharacterMovementComponent.BrakingDecelerationWalking` (`self.Braking Deceleration Walking`) _charactermovement)
      (set `CharacterMovementComponent.GravityScale` (`self.Gravity Scale`) _charactermovement)
      (set `self.Sliding` false)
      (bind (_outhit _returnvalue_2) (`KismetSystemLibrary.LineTraceSingle` _returnvalue (+ _returnvalue (0.0 0.0 450.0)) "TraceTypeQuery1"))
      (if (not _returnvalue_2)
        (`self.OnStartStopCrouch` false)
        (else
          (`self.AdaptiveCrouchCheck`)))
      (`Controller.ResetIgnoreMoveInput` (`GameplayStatics.GetPlayerController` 0))
      (`self.SetComponentTickEnabled` false)
      (`KismetSystemLibrary.Delay` 2.0)
      (set `self.SlideCooldown` false))))

(event `AdaptiveCrouchCheck`
  (`KismetSystemLibrary.K2_SetTimerDelegate` (delegate `CrouchCheckLoop`) 0.1 true))

(event `CrouchCheckLoop`
  (bind _returnvalue (`Actor.K2_GetActorLocation` (`self.GetOwner`)))
  (bind (_outhit _returnvalue_2) (`KismetSystemLibrary.LineTraceSingle` _returnvalue (+ _returnvalue (0.0 0.0 150.0)) "TraceTypeQuery1"))
  (if (not _returnvalue_2)
    (`KismetSystemLibrary.K2_ClearAndInvalidateTimerHandle` (`self.CrouchCheckTimer`))
    (`self.OnStartStopCrouch` false)))

(fn `Check if floor is sloped`
  (params (Vector :type "Vector Structure"))
  (returns (`Flat Ground Vector` :type "Vector Structure"))
  (bind _returnvalue (`KismetMathLibrary.Vector_Up`))
  ; Check if ground is slope to slide
  (if (== Vector _returnvalue :`ErrorTolerance` 0.0001)
    (return (0.0 0.0 0.0))
    (else
      (return (* (`KismetMathLibrary.Normal` (`KismetMathLibrary.Cross_VectorVector` Vector (`KismetMathLibrary.Cross_VectorVector` Vector _returnvalue))) (* (`KismetMathLibrary.FClamp` (- 1.0 (`KismetMathLibrary.Dot_VectorVector` Vector (`KismetMathLibrary.Vector_Up`)))) 500000.0))))))