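; Master actor for pickup weapons, currently holding an unfinished hammer slam attack.
; HammerSlam arms a HammerAttack flag, runs a debug-drawn forward sphere trace whose result is unused, and prints a message.
; While armed, a Box overlap with a BP_MechanicPlayerCharacter clears the flag.
; The DamageMessage call on that character is disconnected, so no damage is dealt.
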(event `self.ReceiveBeginPlay`)

(event `self.Box.OnComponentBeginOverlap`
  (params (OverlappedComponent :type "PrimitiveComponent Object Reference") (OtherActor :type "Actor Object Reference") (OtherComp :type "PrimitiveComponent Object Reference") (OtherBodyIndex :type Integer) (bFromSweep :type Boolean) (SweepResult :type "HitResult Structure (by ref)"))
  (if (`self.HammerAttack?`)
    (bind _asbp_mechanic_player_character (cast `/Game/ThirdPerson/Blueprints/BP_MechanicPlayerCharacter` OtherActor))
    (set `self.HammerAttack?` false)))

(event `HammerSlam`
  (bind _returnvalue (`self.K2_GetActorLocation`))
  ; Make trace cleaner and more accurate for jump shots
  (set `self.HammerAttack?` true)
  (bind _outhit (`KismetSystemLibrary.SphereTraceSingle` :`Start` _returnvalue :`End` (+ _returnvalue (* (`self.GetActorForwardVector`) 500)) :`Radius` 30.0 :`TraceChannel` "TraceTypeQuery1" :`DrawDebugType` "ForDuration"))
  (`KismetSystemLibrary.PrintString` "Slam"))

(fn `UserConstructionScript`)