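; Jelly bean objective actor that scores for the red or blue team when it reaches a King of the Hill jelly bean jar.
; TagRed and TagBlue events set the bean's team as mutually exclusive actor tags.
; When its collision sphere overlaps the jar, it adds points for the tagged team and destroys itself.
; Interact is empty, and the hand-socket pickup and drop logic is left disconnected.
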(event `self.ReceiveBeginPlay`
  (bind _asbp_mechanic_player_character (cast `/Game/ThirdPerson/Blueprints/BP_MechanicPlayerCharacter` (`GameplayStatics.GetPlayerPawn` 0)))
  (set `self.As BP Mechanic Player Character_0` _asbp_mechanic_player_character))

(event `/Game/Blueprints/Interfaces/BPI_Interact.Interact`
  (params (Character :type "/Game/ThirdPerson/Blueprints/BP_MechanicPlayerCharacter Object Reference") (`Character Picking up` :type "/Game/ThirdPerson/Blueprints/BP_MechanicPlayerCharacter Object Reference"))
  ; Interact with bean
)

(event `self.SphereCollsion.OnComponentBeginOverlap`
  (params (OverlappedComponent :type "PrimitiveComponent Object Reference") (OtherActor :type "Actor Object Reference") (OtherComp :type "PrimitiveComponent Object Reference") (OtherBodyIndex :type Integer) (bFromSweep :type Boolean) (SweepResult :type "HitResult Structure (by ref)"))
  ; Changed Jar
  (bind _asbp_jelly_bean_jar_koth (cast `/Game/Blueprints/BP_JellyBeanJarKOTH` OtherActor))
  (`|ExecutionSequence`
    (:`then_0`
      (if (`self.ActorHasTag` "Red")
        (`/Game/Blueprints/BP_JellyBeanJarKOTH.Add Red Bean Points` _asbp_jelly_bean_jar_koth)
        (`self.K2_DestroyActor` :!label _label)))
    (:`then_1`
      (if (`self.ActorHasTag` "Blue")
        (`/Game/Blueprints/BP_JellyBeanJarKOTH.Add Blue Bean points` _asbp_jelly_bean_jar_koth)
        (goto _label)))))

(event `TagRed`
  (bind _tags (`self.Tags`))
  (`KismetArrayLibrary.Array_Add` _tags "Red")
  (`KismetArrayLibrary.Array_RemoveItem` _tags "Blue"))

(event `TagBlue`
  (bind _tags (`self.Tags`))
  (`KismetArrayLibrary.Array_Add` _tags "Blue")
  (`KismetArrayLibrary.Array_RemoveItem` _tags "Red"))

(fn `UserConstructionScript`)