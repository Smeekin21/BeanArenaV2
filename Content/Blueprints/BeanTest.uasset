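; BeanTest is a team-tagged bean actor that scores when its collision sphere overlaps a KOTH jelly bean jar.
; TagRed and TagBlue swap its team tag, which selects the jar's red or blue points call.
; Scoring clears the matching player's thrown and holding flags through BP_ThirdPersonGameMode, then destroys the bean.
; Interact is empty, and the older pickup, attach and drop logic is left unconnected.
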(event `self.ReceiveBeginPlay`
  (bind _asbp_mechanic_player_character (cast `/Game/ThirdPerson/Blueprints/BP_MechanicPlayerCharacter` (`GameplayStatics.GetPlayerPawn` 0)))
  (set `self.As BP Mechanic Player Character_0` _asbp_mechanic_player_character)
  (bind _asbp_third_person_game_mode (cast `/Game/ThirdPerson/Blueprints/BP_ThirdPersonGameMode` (`GameplayStatics.GetGameMode`)))
  (set `self.As BP Third Person Game Mode` _asbp_third_person_game_mode))

(event `self.Interact`
  (params (Character :type "/Game/ThirdPerson/Blueprints/BP_MechanicPlayerCharacter Object Reference") (`Character Picking up` :type "/Game/ThirdPerson/Blueprints/BP_MechanicPlayerCharacter Object Reference"))
  ; Interact with bean
)

(event `self.SphereCollsion.OnComponentBeginOverlap`
  (params (OverlappedComponent :type "PrimitiveComponent Object Reference") (OtherActor :type "Actor Object Reference") (OtherComp :type "PrimitiveComponent Object Reference") (OtherBodyIndex :type Integer) (bFromSweep :type Boolean) (SweepResult :type "HitResult Structure (by ref)"))
  (bind _as_bp_third_person_game_mode (`self.As BP Third Person Game Mode`))
  (bind _firstplayercharacter (`/Game/ThirdPerson/Blueprints/BP_ThirdPersonGameMode.FirstPlayerCharacter` _as_bp_third_person_game_mode))
  (bind _secondplayercharacter (`/Game/ThirdPerson/Blueprints/BP_ThirdPersonGameMode.SecondPlayerCharacter` _as_bp_third_person_game_mode))
  ; Changed Jar
  (bind _asbp_jelly_bean_jar_koth (cast `/Game/Blueprints/BP_JellyBeanJarKOTH` OtherActor))
  (`|ExecutionSequence`
    (:`then_0`
      (if (`self.ActorHasTag` "Red")
        (`/Game/Blueprints/BP_JellyBeanJarKOTH.Add Red Bean Points` _asbp_jelly_bean_jar_koth)
        (set `/Game/ThirdPerson/Blueprints/BP_MechanicPlayerCharacter.Thrown?` false _firstplayercharacter)
        (set `/Game/ThirdPerson/Blueprints/BP_MechanicPlayerCharacter.HoldingBean?` false _firstplayercharacter)
        (set `/Game/ThirdPerson/Blueprints/BP_MechanicPlayerCharacter.Holding Item?` false _firstplayercharacter)
        (`self.K2_DestroyActor` :!label _label)))
    (:`then_1`
      (if (`self.ActorHasTag` "Blue")
        (`/Game/Blueprints/BP_JellyBeanJarKOTH.Add Blue Bean points` _asbp_jelly_bean_jar_koth)
        (set `/Game/ThirdPerson/Blueprints/BP_MechanicPlayerCharacter.Thrown?` false _secondplayercharacter)
        (set `/Game/ThirdPerson/Blueprints/BP_MechanicPlayerCharacter.HoldingBean?` false _secondplayercharacter)
        (set `/Game/ThirdPerson/Blueprints/BP_MechanicPlayerCharacter.Holding Item?` false _secondplayercharacter)
        (goto _label)))))

(event `TagRed`
  (bind _tags (`self.Tags`))
  (`KismetArrayLibrary.Array_Add` _tags "Red")
  (`KismetArrayLibrary.Array_RemoveItem` _tags "Blue"))

(event `TagBlue`
  (bind _tags (`self.Tags`))
  (`KismetArrayLibrary.Array_Add` _tags "Blue")
  (`KismetArrayLibrary.Array_RemoveItem` _tags "Red"))

(fn `UserConstructionScript`)