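; Short-lived jelly bean projectile with rocket-jump knockback and power-up variants, whose gravity increases shortly after spawn.
; On BeginPlay it reads flags from the first player character found: explosive runs a delayed sphere-trace damage burst, bullet increase spawns child beans via a timeline.
; Sphere hits pop the player character upward unless aiming, and launch the owner set by SetOwningPlayer away from nearby impacts.
; Older hit-damage experiments remain disconnected.
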(event `EnhancedInput|/Game/Input/Actions/IA_BeanThrow`
  (params (ActionValue :type Boolean) (ElapsedSeconds :type "Float (double-precision)") (TriggeredSeconds :type "Float (double-precision)") (InputAction :type "InputAction Object Reference" :default "/Game/Input/Actions/IA_BeanThrow.IA_BeanThrow"))
  ; Grenade throw
)

(event `EnhancedInput|/Game/Input/Actions/Shield/IA_Throw`
  (params (ActionValue :type Boolean) (ElapsedSeconds :type "Float (double-precision)") (TriggeredSeconds :type "Float (double-precision)") (InputAction :type "InputAction Object Reference" :default "/Game/Input/Actions/Shield/IA_Throw.IA_Throw"))
  ; Grenade throw
)

(event `self.ReceiveBeginPlay`
  (bind _returnvalue (`self.K2_GetActorLocation`))
  (bind (_returnvalue_location _returnvalue_rotation) (`KismetMathLibrary.BreakTransform` (`self.GetTransform`)))
  (bind _asbp_third_person_game_mode (cast `/Game/ThirdPerson/Blueprints/BP_ThirdPersonGameMode` (`GameplayStatics.GetGameMode`)))
  (set `self.As BP Third Person Game Mode` _asbp_third_person_game_mode)
  (`|ExecutionSequence`
    (:`then_0`
      (bind _returnvalue_2 (`GameplayStatics.GetActorOfClass` "/Game/ThirdPerson/Blueprints/BP_MechanicPlayerCharacter.BP_MechanicPlayerCharacter_C"))
      (set `self.Player Ref` _returnvalue_2)
      (`self.SetLifeSpan` 1.0)
      (`|ExecutionSequence`
        (:`then_0`
          (if (`/Game/ThirdPerson/Blueprints/BP_MechanicPlayerCharacter.ExplosivePowerUp?` _returnvalue_2)
            (`KismetSystemLibrary.Delay` 0.8)
            (bind _outhits (`KismetSystemLibrary.SphereTraceMulti` :`Start` _returnvalue :`End` _returnvalue :`Radius` 150.0 :`TraceChannel` "TraceTypeQuery1" :`DrawDebugType` "ForDuration" :`bIgnoreSelf` false))
            (for _array_element _outhits
              (`GameplayStatics.SpawnEmitterAtLocation` "/Engine/Tutorial/SubEditors/TutorialAssets/TutorialParticleSystem.TutorialParticleSystem")
              (bind (_bblockinghit _binitialoverlap _time _distance _location _impactpoint _normal _impactnormal _physmat _hitactor) (`GameplayStatics.BreakHitResult` _array_element))
              (message `/Game/Blueprints/Interfaces/BPI_Damage.Damage` _hitactor 20.0 0.0 false _hitactor))))
        (:`then_1`
          (if (`/Game/ThirdPerson/Blueprints/BP_MechanicPlayerCharacter.Bullet Increase Powerup?` _returnvalue_2)
            (`/Engine/EditorBlueprintResources/StandardMacros.DoOnce` false
              (:`Completed`
                (`Timeline|Timeline`
                  (:`Spawn`
                    (`|SpawnActorFromClass` "/Game/Blueprints/BP_JellyBean_Projectile_Child.BP_JellyBean_Projectile_Child_C" (`KismetMathLibrary.MakeTransform` _returnvalue_location _returnvalue_rotation (0.75 0.75 0.75)) "AlwaysSpawn" "MultiplyWithRoot" null null null)))))))))
    (:`then_1`
      (`KismetSystemLibrary.Delay` 0.1)
      (set `ProjectileMovementComponent.ProjectileGravityScale` 5.0 (`self.ProjectileMovement`)))))

(event `self.Capsule.OnComponentBeginOverlap`
  (params (OverlappedComponent :type "PrimitiveComponent Object Reference") (OtherActor :type "Actor Object Reference") (OtherComp :type "PrimitiveComponent Object Reference") (OtherBodyIndex :type Integer) (bFromSweep :type Boolean) (SweepResult :type "HitResult Structure (by ref)")))

(event `self.Sphere.OnComponentHit`
  (params (HitComponent :type "PrimitiveComponent Object Reference") (OtherActor :type "Actor Object Reference") (OtherComp :type "PrimitiveComponent Object Reference") (NormalImpulse :type "Vector Structure") (Hit :type "HitResult Structure (by ref)"))
  (bind (_bblockinghit _binitialoverlap _time _distance _location _impactpoint) (`GameplayStatics.BreakHitResult` Hit))
  (bind _owner_0 (`self.Owner_0`))
  (bind _returnvalue (`self.K2_GetActorLocation` _owner_0))
  (`|ExecutionSequence`
    (:`then_0`
      ; Rocket Jump Movement Ability
      (bind _asbp_mechanic_player_character (cast `/Game/ThirdPerson/Blueprints/BP_MechanicPlayerCharacter` OtherActor))
      (set `self.As BP Mechanic Player Character` _asbp_mechanic_player_character)
      (`/Engine/EditorBlueprintResources/StandardMacros.DoOnce` false :!label _label
        (:`Completed`
          (if (== OtherActor (`self.Player Ref`))
            (if (`/Game/ThirdPerson/Blueprints/BP_MechanicPlayerCharacter.Aiming?` _asbp_mechanic_player_character)
              (`Character.LaunchCharacter` _asbp_mechanic_player_character (0.0 0.0 0.0) false false)
              (else
                (`Character.LaunchCharacter` _asbp_mechanic_player_character (0.0 0.0 900.0) false false)))
            (`KismetSystemLibrary.Delay` 2.0)
            (goto _label :!via `Reset`)))))
    (:`then_1`
      ; Rocket Sphere trace for if character should launch up
      (if _bblockinghit
        (`/Engine/EditorBlueprintResources/StandardMacros.DoOnce` false
          (:`Completed`
            ;; Make valid some how
            (`/Engine/EditorBlueprintResources/StandardMacros.IsValid` _owner_0
              (:`Is Valid`
                (if (<= (`KismetMathLibrary.Vector_Distance` _impactpoint _returnvalue) 500.0)
                  (`/Engine/EditorBlueprintResources/StandardMacros.IsValid` _owner_0
                    (:`Is Valid`
                      (`Character.LaunchCharacter` _owner_0 (* (`KismetMathLibrary.GetDirectionUnitVector` _impactpoint _returnvalue) 1800) true true))))))))))))

(event `SetOwningPlayer`
  (params (Owner :type "/Game/ThirdPerson/Blueprints/BP_MechanicPlayerCharacter Object Reference"))
  (set `self.Owner_0` Owner))

(event `Explosive_Powerup_Upgrade`
  (bind _as_bp_mechanic_player_character (`self.As BP Mechanic Player Character`))
  (`/Engine/EditorBlueprintResources/StandardMacros.FlipFlop`
    (:`A`
      (set `/Game/ThirdPerson/Blueprints/BP_MechanicPlayerCharacter.ExplosivePowerUp?` true _as_bp_mechanic_player_character))
    (:`B`
      (set `/Game/ThirdPerson/Blueprints/BP_MechanicPlayerCharacter.ExplosivePowerUp?` false _as_bp_mechanic_player_character))))

(event `/Game/Blueprints/Interfaces/BPI_Damage.Damage`
  (params (`Damage Amount` :type "Float (double-precision)") (CurrentHealth :type "Float (double-precision)") (`IsDead?` :type Boolean) (Target :type "Actor Object Reference"))
  (bind _as_bp_mechanic_player_character (`self.As BP Mechanic Player Character`))
  (`KismetSystemLibrary.PrintString` "Hello")
  (`/Engine/EditorBlueprintResources/StandardMacros.IsValid` _as_bp_mechanic_player_character
    (:`Is Valid`
      (set `/Game/ThirdPerson/Blueprints/BP_MechanicPlayerCharacter.Current Health` (- `Damage Amount` 20.0) _as_bp_mechanic_player_character))
    (:`Is Not Valid`
      (`KismetSystemLibrary.PrintString` "AGHH"))))

(event `Bullet Increase Powerup`
  (bind _as_bp_mechanic_player_character (`self.As BP Mechanic Player Character`))
  (`/Engine/EditorBlueprintResources/StandardMacros.FlipFlop`
    (:`A`
      (set `/Game/ThirdPerson/Blueprints/BP_MechanicPlayerCharacter.Bullet Increase Powerup?` true _as_bp_mechanic_player_character))
    (:`B`
      (set `/Game/ThirdPerson/Blueprints/BP_MechanicPlayerCharacter.Bullet Increase Powerup?` false _as_bp_mechanic_player_character))))

(fn `Explosive Bullet`
  (bind _returnvalue (`self.K2_GetActorLocation`))
  (bind _outhits (`KismetSystemLibrary.SphereTraceMulti` :`Start` _returnvalue :`End` _returnvalue :`Radius` 150.0 :`TraceChannel` "TraceTypeQuery1" :`DrawDebugType` "ForDuration" :`bIgnoreSelf` false))
  (for _array_element _outhits
    (bind (_bblockinghit _binitialoverlap _time _distance _location _impactpoint _normal _impactnormal _physmat _hitactor) (`GameplayStatics.BreakHitResult` _array_element))
    (if _bblockinghit
      (`KismetSystemLibrary.PrintString` (`KismetSystemLibrary.GetDisplayName` _hitactor))
      (bind _returnvalue_2 (`self.ActorHasTag` _hitactor "Explodes"))
      (if _returnvalue_2
        (`KismetSystemLibrary.PrintString` (`KismetStringLibrary.Conv_BoolToString` _returnvalue_2))
        (`GameplayStatics.SpawnEmitterAtLocation` "/Engine/Tutorial/SubEditors/TutorialAssets/TutorialParticleSystem.TutorialParticleSystem" _returnvalue)
        (`/Game/Blueprints/Interfaces/BPI_Damage.Damage` 20.0 0.0 false _hitactor)))))

(fn `UserConstructionScript`)