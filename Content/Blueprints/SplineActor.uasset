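; SplineActor is a hazard actor that moves a static mesh along a spline and damages the player character on contact.
; On BeginPlay, a timeline scales its track value by the spline length and places the mesh at that world-space distance each update, without sweeping.
; A Box overlap casts the other actor to BP_MechanicPlayerCharacter and calls Damage with a very large amount.
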(event `self.ReceiveBeginPlay`
  (bind (_direction _timetrack) (`Timeline|Timeline`)
    (:`Update`
      (`SceneComponent.K2_SetWorldLocation` (`self.StaticMesh`) (`SplineComponent.GetLocationAtDistanceAlongSpline` (`self.Spline`) (* _timetrack (`SplineComponent.GetSplineLength` (`self.Spline`))) "World") false false))))

(event `self.Box.OnComponentBeginOverlap`
  (params (OverlappedComponent :type "PrimitiveComponent Object Reference") (OtherActor :type "Actor Object Reference") (OtherComp :type "PrimitiveComponent Object Reference") (OtherBodyIndex :type Integer) (bFromSweep :type Boolean) (SweepResult :type "HitResult Structure (by ref)"))
  (bind _asbp_mechanic_player_character (cast `/Game/ThirdPerson/Blueprints/BP_MechanicPlayerCharacter` OtherActor))
  (`/Game/Blueprints/Interfaces/BPI_Damage.Damage` _asbp_mechanic_player_character 10000.0 0.0 false null))

(fn `UserConstructionScript`)