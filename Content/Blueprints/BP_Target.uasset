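; Shootable-style target actor that changes material as it takes damage and destroys itself when its health runs out.
; The Damage event ignores the damage amount and subtracts one from CurrentHealth per hit.
; A Sequence runs three macros that each match a health value of 3, 2 or 1 to set the material.
; Each branch then repeats the death check, which assigns IsDead to itself before destroying the actor.
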(event `/Game/Blueprints/Interfaces/BPI_Damage.Damage`
  (params (`Damage Amount` :type "Float (double-precision)") (CurrentHealth :type "Float (double-precision)") (`IsDead?` :type Boolean) (Target :type "Actor Object Reference"))
  (bind _output_get (set `self.Current Health` (- (`self.Current Health`) 1.0)))
  (`|ExecutionSequence`
    (:`then_0`
      (if (== (`self.Current Health`) 3.0)
        (`PrimitiveComponent.SetMaterial` (`self.Target`) 0 "/Niagara/DefaultAssets/GeometryCache/M_DefaultGeometryCacheMaterial_Green.M_DefaultGeometryCacheMaterial_Green")))
    (:`then_1`
      (if (== (`self.Current Health`) 2.0)
        (`PrimitiveComponent.SetMaterial` (`self.Target`) 0 "/Engine/Tutorial/SubEditors/TutorialAssets/Character/TutorialTPP_Mat.TutorialTPP_Mat")))
    (:`then_2`
      (if (== (`self.Current Health`) 1.0)
        (`PrimitiveComponent.SetMaterial` (`self.Target`) 0 "/Engine/VREditor/BasicMeshes/MI_Cube_03.MI_Cube_03"))))
  (if (<= _output_get 0.0)
    (set `self.Is Dead?` (`self.Is Dead?`))
    (`self.K2_DestroyActor`)))

(fn `UserConstructionScript`)