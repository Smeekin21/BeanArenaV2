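; Jelly bean jar that tracks and displays red and blue bean points for two players.
; Add-point events increment that color's count on both player characters, then bump the jar's counter, which switches to reveal the next of five bean meshes per color.
; BeginPlay runs both counter bumps too, and cylinder overlaps briefly change the overlay material's draw distance.
; Interact is empty; older deposit, take and spawn logic is disconnected.
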(event `self.ReceiveBeginPlay`
  (`self.Set beans visible`)
  (`self.Set Blue beans visible`)
  (set `self.BeansInJarArray` (`self.BeansInJarArray`)))

(event `/Game/Blueprints/Interfaces/BPI_Interact.Interact`
  (params (Character :type "/Game/ThirdPerson/Blueprints/BP_MechanicPlayerCharacter Object Reference") (`Character Picking up` :type "/Game/ThirdPerson/Blueprints/BP_MechanicPlayerCharacter Object Reference")))

(event `Set Blue beans visible`
  (bind _bean6 (`self.Bean6`))
  (bind _bean7 (`self.Bean7`))
  (bind _bean8 (`self.Bean8`))
  (bind _bean9 (`self.Bean9`))
  (bind _bean10 (`self.Bean10`))
  ;[0 0.5989 0.9281 0.5] Setting Blue beans visible
  (`KismetArrayLibrary.Array_Clear` (`self.BeansInJarArray`))
  (`|ExecutionSequence`
    (:`then_0`
      (`/Engine/EditorBlueprintResources/StandardMacros.IncrementInt` (`self.Blue Beans in Jar`)
        (:`  `
          (switch `int` (`self.Blue Beans in Jar`)
            (:`0`
              (`self.Empty Jar`))
            (:`1`
              (`KismetArrayLibrary.Array_Add` (`self.BeansInJarArray`) _bean6)
              (`SceneComponent.SetVisibility` _bean6 true false))
            (:`2`
              (`KismetArrayLibrary.Array_Add` (`self.BeansInJarArray`) _bean7)
              (`SceneComponent.SetVisibility` _bean7 true false))
            (:`3`
              (`KismetArrayLibrary.Array_Add` (`self.BeansInJarArray`) _bean8)
              (`SceneComponent.SetVisibility` _bean8 true false))
            (:`4`
              (`KismetArrayLibrary.Array_Add` (`self.BeansInJarArray`) _bean9)
              (`SceneComponent.SetVisibility` _bean9 true false))
            (:`5`
              (`KismetArrayLibrary.Array_Add` (`self.BeansInJarArray`) _bean10)
              (`SceneComponent.SetVisibility` _bean10 true false))))))
    (:`then_1`
      (if (not (`self.empty?`))
        (for _array_element (`self.BeansInJarArray`)
          (`SceneComponent.SetVisibility` _array_element true false))))))

(event `Set beans visible`
  (bind _bean2 (`self.Bean2`))
  (bind _bean3 (`self.Bean3`))
  (bind _bean4 (`self.Bean4`))
  (bind _bean5 (`self.Bean5`))
  ;[1 0.01137 0 0.5] Setting Red Beans Visible
  (`KismetArrayLibrary.Array_Clear` (`self.BeansInJarArray`))
  (`|ExecutionSequence`
    (:`then_0`
      (`/Engine/EditorBlueprintResources/StandardMacros.IncrementInt` (`self.Beans in Jar`)
        (:`  `
          (switch `int` (`self.Beans in Jar`)
            (:`0`
              (`self.Empty Jar`))
            (:`1`
              (`KismetArrayLibrary.Array_Add` (`self.BeansInJarArray`) (`self.Bean1`))
              (`SceneComponent.SetVisibility` (`self.Bean1`) true false))
            (:`2`
              (`KismetArrayLibrary.Array_Add` (`self.BeansInJarArray`) _bean2)
              (`SceneComponent.SetVisibility` _bean2 true false))
            (:`3`
              (`KismetArrayLibrary.Array_Add` (`self.BeansInJarArray`) _bean3)
              (`SceneComponent.SetVisibility` _bean3 true false))
            (:`4`
              (`KismetArrayLibrary.Array_Add` (`self.BeansInJarArray`) _bean4)
              (`SceneComponent.SetVisibility` _bean4 true false))
            (:`5`
              (`KismetArrayLibrary.Array_Add` (`self.BeansInJarArray`) _bean5)
              (`SceneComponent.SetVisibility` _bean5 true false))))))
    (:`then_1`
      (if (not (`self.empty?`))
        (for _array_element (`self.BeansInJarArray`)
          (`SceneComponent.SetVisibility` _array_element true false))))))

(event `self.Cylinder.OnComponentBeginOverlap`
  (params (OverlappedComponent :type "PrimitiveComponent Object Reference") (OtherActor :type "Actor Object Reference") (OtherComp :type "PrimitiveComponent Object Reference") (OtherBodyIndex :type Integer) (bFromSweep :type Boolean) (SweepResult :type "HitResult Structure (by ref)"))
  ; Point Added
  (`MeshComponent.SetOverlayMaterialMaxDrawDistance` (`self.Cylinder`) 0.0)
  (`KismetSystemLibrary.Delay` 0.5)
  (`MeshComponent.SetOverlayMaterialMaxDrawDistance` (`self.Cylinder`) 1.0))

(event `Add Red Bean Points`
  (bind _asbp_mechanic_player_character (cast `/Game/ThirdPerson/Blueprints/BP_MechanicPlayerCharacter` (`GameplayStatics.GetPlayerPawn` 0)))
  (`/Engine/EditorBlueprintResources/StandardMacros.IncrementInt` (`/Game/ThirdPerson/Blueprints/BP_MechanicPlayerCharacter.Red Beans` _asbp_mechanic_player_character)
    (:`  `
      (bind _asbp_mechanic_player_character_2 (cast `/Game/ThirdPerson/Blueprints/BP_MechanicPlayerCharacter` (`GameplayStatics.GetPlayerPawn` 1)))
      (`/Engine/EditorBlueprintResources/StandardMacros.IncrementInt` (`/Game/ThirdPerson/Blueprints/BP_MechanicPlayerCharacter.Red Beans` _asbp_mechanic_player_character_2)
        (:`  `
          (`self.Set beans visible`))))))

(event `Add Blue Bean points`
  (bind _asbp_mechanic_player_character (cast `/Game/ThirdPerson/Blueprints/BP_MechanicPlayerCharacter` (`GameplayStatics.GetPlayerPawn` 0)))
  (`/Engine/EditorBlueprintResources/StandardMacros.IncrementInt` (`/Game/ThirdPerson/Blueprints/BP_MechanicPlayerCharacter.Blue Beans` _asbp_mechanic_player_character)
    (:`  `
      (bind _asbp_mechanic_player_character_2 (cast `/Game/ThirdPerson/Blueprints/BP_MechanicPlayerCharacter` (`GameplayStatics.GetPlayerPawn` 1)))
      (`/Engine/EditorBlueprintResources/StandardMacros.IncrementInt` (`/Game/ThirdPerson/Blueprints/BP_MechanicPlayerCharacter.Blue Beans` _asbp_mechanic_player_character_2)
        (:`  `
          (`self.Set Blue beans visible`))))))

(fn `UserConstructionScript`)