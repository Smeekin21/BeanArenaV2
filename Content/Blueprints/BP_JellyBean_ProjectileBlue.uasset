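; Blue jelly bean projectile with a short lifespan that provides a rocket jump for the player who fired it.
; Sphere hits launch the owner away from nearby impacts and set their cooldown; distant blocking impacts destroy the projectile.
; A direct-hit vertical launch depends on PlayerRef, which only disconnected code assigns.
; Powerup events toggle character flags, but explosive traces, child-projectile spawning and enemy damage logic are unwired or uncalled here.
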(event `EnhancedInput|/Game/Input/Actions/IA_BeanThrow`
  (params (ActionValue :type Boolean) (ElapsedSeconds :type "Float (double-precision)") (TriggeredSeconds :type "Float (double-precision)") (InputAction :type "InputAction Object Reference" :default "/Game/Input/Actions/IA_BeanThrow.IA_BeanThrow"))
  ; Grenade throw
)

(event `EnhancedInput|/Game/Input/Actions/Shield/IA_Throw`
  (params (ActionValue :type Boolean) (ElapsedSeconds :type "Float (double-precision)") (TriggeredSeconds :type "Float (double-precision)") (InputAction :type "InputAction Object Reference" :default "/Game/Input/Actions/Shield/IA_Throw.IA_Throw"))
  ; Grenade throw
)

(event `self.ReceiveBeginPlay`
  (bind _returnvalue (`self.GetOwner`))
  (`self.SetLifeSpan` 2.0)
  (if (== _returnvalue (`/Game/ThirdPerson/Blueprints/BP_ThirdPersonGameMode.FirstPlayerCharacter` (`self.As BP Third Person Game Mode`)))
    (cast `/Game/ThirdPerson/Blueprints/BP_MechanicPlayerCharacter` _returnvalue)
    (`KismetSystemLibrary.PrintString` "Player1")
    (elif (== (`self.GetOwner`) (`/Game/ThirdPerson/Blueprints/BP_ThirdPersonGameMode.SecondPlayerCharacter` (`self.As BP Third Person Game Mode`)))
      (cast `/Game/ThirdPerson/Blueprints/BP_MechanicPlayerCharacter` _returnvalue)
      (`KismetSystemLibrary.PrintString` "Player2"))))

(event `self.Capsule.OnComponentBeginOverlap`
  (params (OverlappedComponent :type "PrimitiveComponent Object Reference") (OtherActor :type "Actor Object Reference") (OtherComp :type "PrimitiveComponent Object Reference") (OtherBodyIndex :type Integer) (bFromSweep :type Boolean) (SweepResult :type "HitResult Structure (by ref)")))

(event `self.Sphere.OnComponentHit`
  (params (HitComponent :type "PrimitiveComponent Object Reference") (OtherActor :type "Actor Object Reference") (OtherComp :type "PrimitiveComponent Object Reference") (NormalImpulse :type "Vector Structure") (Hit :type "HitResult Structure (by ref)"))
  (bind (_bblockinghit _binitialoverlap _time _distance _location _impactpoint) (`GameplayStatics.BreakHitResult` Hit))
  (bind _projectileowner (`self.ProjectileOwner`))
  (bind _returnvalue (`self.K2_GetActorLocation` _projectileowner))
  (`|ExecutionSequence`
    (:`then_0`
      ; Rocket Jump Movement Ability
      (bind _asbp_mechanic_player_character (cast `/Game/ThirdPerson/Blueprints/BP_MechanicPlayerCharacter` OtherActor))
      (set `self.As BP Mechanic Player Character` _asbp_mechanic_player_character)
      (`/Engine/EditorBlueprintResources/StandardMacros.DoOnce` false :!label _label
        (:`Completed`
          (if (== OtherActor (`self.Player Ref`))
            (if (`/Game/ThirdPerson/Blueprints/BP_MechanicPlayerCharacter.Aiming?` _asbp_mechanic_player_character)
              (`Character.LaunchCharacter` _asbp_mechanic_player_character (0.0 0.0 0.0) false false)
              (else
                (`Character.LaunchCharacter` _asbp_mechanic_player_character (0.0 0.0 900.0) false false)))
            (`KismetSystemLibrary.Delay` 2.0)
            (goto _label :!via `Reset`)))))
    (:`then_1`
      (if (not (`/Game/ThirdPerson/Blueprints/BP_MechanicPlayerCharacter.RocketJumpCooldown` (`self.ProjectileOwner`)))
        ; Rocket Sphere trace for if character should launch up
        (if _bblockinghit
          (`/Engine/EditorBlueprintResources/StandardMacros.DoOnce` false
            (:`Completed`
              ;; Make valid some how
              (`/Engine/EditorBlueprintResources/StandardMacros.IsValid` _projectileowner
                (:`Is Valid`
                  (if (<= (`KismetMathLibrary.Vector_Distance` _impactpoint _returnvalue) 400.0)
                    (`/Engine/EditorBlueprintResources/StandardMacros.IsValid` _projectileowner
                      (:`Is Valid`
                        (`Character.LaunchCharacter` _projectileowner (* (`KismetMathLibrary.GetDirectionUnitVector` _impactpoint _returnvalue) 1250) false true)
                        (set `/Game/ThirdPerson/Blueprints/BP_MechanicPlayerCharacter.RocketJumpCooldown` true _projectileowner)))
                    (else
                      (`KismetSystemLibrary.PrintString` "Not it")
                      (`self.K2_DestroyActor`))))))))))))

(event `SetOwningPlayer`
  (params (Owner :type "/Game/ThirdPerson/Blueprints/BP_MechanicPlayerCharacter Object Reference"))
  (set `self.ProjectileOwner` Owner))

(event `Explosive_Powerup_Upgrade`
  (bind _as_bp_mechanic_player_character (`self.As BP Mechanic Player Character`))
  (`/Engine/EditorBlueprintResources/StandardMacros.FlipFlop`
    (:`A`
      (set `/Game/ThirdPerson/Blueprints/BP_MechanicPlayerCharacter.ExplosivePowerUp?` true _as_bp_mechanic_player_character))
    (:`B`
      (set `/Game/ThirdPerson/Blueprints/BP_MechanicPlayerCharacter.ExplosivePowerUp?` false _as_bp_mechanic_player_character))))

(event `self.Damage`
  (params (`Damage Amount` :type "Float (double-precision)") (CurrentHealth :type "Float (double-precision)") (`IsDead?` :type Boolean) (Target :type "Actor Object Reference"))
  (bind _as_bp_mechanic_player_character (`self.As BP Mechanic Player Character`))
  (`KismetSystemLibrary.PrintString` "Hello")
  (`/Engine/EditorBlueprintResources/StandardMacros.IsValid` _as_bp_mechanic_player_character
    (:`Is Valid`
      (set `/Game/ThirdPerson/Blueprints/BP_MechanicPlayerCharacter.Current Health` (- `Damage Amount` 20.0) _as_bp_mechanic_player_character))
    (:`Is Not Valid`
      (`KismetSystemLibrary.PrintString` "AGHH"))))

(event `Bullet Increase Powerup`
  (bind _as_bp_mechanic_player_character (`self.As BP Mechanic Player Character`))
  (`/Engine/EditorBlueprintResources/StandardMacros.FlipFlop`
    (:`A`
      (set `/Game/ThirdPerson/Blueprints/BP_MechanicPlayerCharacter.Bullet Increase Powerup?` true _as_bp_mechanic_player_character))
    (:`B`
      (set `/Game/ThirdPerson/Blueprints/BP_MechanicPlayerCharacter.Bullet Increase Powerup?` false _as_bp_mechanic_player_character))))

(fn `Explosive Bullet`
  (bind _returnvalue (`self.K2_GetActorLocation`))
  (bind _outhits (`KismetSystemLibrary.SphereTraceMulti` :`Start` _returnvalue :`End` _returnvalue :`Radius` 150.0 :`TraceChannel` "TraceTypeQuery1" :`DrawDebugType` "ForDuration" :`bIgnoreSelf` false))
  (for _array_element _outhits
    (bind (_bblockinghit _binitialoverlap _time _distance _location _impactpoint _normal _impactnormal _physmat _hitactor) (`GameplayStatics.BreakHitResult` _array_element))
    (if _bblockinghit
      (`KismetSystemLibrary.PrintString` (`KismetSystemLibrary.GetDisplayName` _hitactor))
      (bind _returnvalue_2 (`self.ActorHasTag` _hitactor "Explodes"))
      (if _returnvalue_2
        (`KismetSystemLibrary.PrintString` (`KismetStringLibrary.Conv_BoolToString` _returnvalue_2))
        (`GameplayStatics.SpawnEmitterAtLocation` "/Engine/Tutorial/SubEditors/TutorialAssets/TutorialParticleSystem.TutorialParticleSystem" _returnvalue)
        (`/Game/Blueprints/Interfaces/BPI_Damage.Damage` 20.0 0.0 false _hitactor)))))

(fn `UserConstructionScript`)