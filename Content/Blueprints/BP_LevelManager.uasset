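; Level manager that times jelly bean jar rounds and declares a winner between two players.
; A per-round delay leads to a timer that spawns a scaled-up jar at the manager's location.
; Parallel delays in the spawn event hide the jar and increment the round, mostly restarting the cycle.
; Tick polls a jar's two bean counters, showing that player's win widget and pausing at five beans.
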(event `Countdown`
  ;[0.3112 0.7906 0.1018 0.5] Countdown Timer
  (switch `int` (`self.RoundNumber`)
    (:`0`
      (if (<= (`self.FirstSpawn`) 10.0)
        (bind _returnvalue (`KismetSystemLibrary.K2_SetTimerDelegate` (delegate `JarSpawnRounds`) (`self.CountdownTime`) :!label _label))
        (set `self.CountdownTimer` _returnvalue)))
    (:`1`
      (if (<= (`self.SecondSpawn`) 10.0)
        (goto _label)))
    (:`2`
      (if (<= (`self.ThirdSpawn`) 10.0)
        (goto _label)))
    (:`3`
      (if (<= (`self.FourthSpawn`) 10.0)
        (goto _label)))
    (:`4`
      (if (<= (`self.FifthSpawn`) 10.0)
        (goto _label)))))

(event `self.ReceiveBeginPlay`
  (`|ExecutionSequence`
    (:`then_0`
      (bind _asbp_mechanic_player_character (cast `/Game/ThirdPerson/Blueprints/BP_MechanicPlayerCharacter` (`GameplayStatics.GetPlayerCharacter` 0)))
      (set `self.As BP Mechanic Player Character` _asbp_mechanic_player_character))
    (:`then_1`
      (switch `int` (`self.RoundNumber`) :!label _label_2
        (:`0`
          (`KismetSystemLibrary.Delay` (`self.FirstSpawn`))
          (`KismetSystemLibrary.PrintString` "Countimg")
          (`self.Countdown`))
        (:`1`
          (`KismetSystemLibrary.Delay` (`self.SecondSpawn`))
          (`self.Countdown`))
        (:`2`
          (`KismetSystemLibrary.Delay` (`self.ThirdSpawn`))
          (`self.Countdown`))
        (:`3`
          (`KismetSystemLibrary.Delay` (`self.FourthSpawn`))
          (`self.Countdown`))
        (:`4`
          (`KismetSystemLibrary.Delay` (`self.FifthSpawn`))
          (`self.Countdown`))))))

(event `JarSpawnRounds`
  (bind _returnvalue_location (`KismetMathLibrary.BreakTransform` (`self.GetTransform`)))
  (`|ExecutionSequence`
    (:`then_0`
      (bind _returnvalue (`|SpawnActorFromClass` "/Game/Blueprints/BP_JellyBeanJar.BP_JellyBeanJar_C" (`KismetMathLibrary.MakeTransform` _returnvalue_location (struct) (5.0 5.0 5.0)) "AlwaysSpawn" "MultiplyWithRoot" null null))
      (bind _output_get (set `self.Jar` _returnvalue))
      (`KismetSystemLibrary.Delay` (`self.FirstRoundCount`))
      (`self.SetActorHiddenInGame` _output_get true)
      (`/Engine/EditorBlueprintResources/StandardMacros.IncrementInt` (`self.RoundNumber`)
        (:`  `
          (`self.AnotherRound`))))
    (:`then_1`
      (`KismetSystemLibrary.Delay` (`self.SecondRoundCount`))
      (`self.SetActorHiddenInGame` (`self.Jar`) true)
      (`/Engine/EditorBlueprintResources/StandardMacros.IncrementInt` (`self.RoundNumber`)
        (:`  `
          (`self.AnotherRound`))))
    (:`then_2`
      (`KismetSystemLibrary.Delay` (`self.ThirdSpawn`))
      (`self.SetActorHiddenInGame` (`self.Jar`) true)
      (`/Engine/EditorBlueprintResources/StandardMacros.IncrementInt` (`self.RoundNumber`)
        (:`  `
          (`self.AnotherRound`))))
    (:`then_3`
      (`KismetSystemLibrary.Delay` (`self.FourthSpawn`))
      (`self.SetActorHiddenInGame` (`self.Jar`) true)
      (`/Engine/EditorBlueprintResources/StandardMacros.IncrementInt` (`self.RoundNumber`)
        (:`  `
          (`self.AnotherRound`))))
    (:`then_4`
      (`KismetSystemLibrary.Delay` (`self.FifthSpawn`))
      (`self.SetActorHiddenInGame` (`self.Jar`) true)
      (`/Engine/EditorBlueprintResources/StandardMacros.IncrementInt` (`self.RoundNumber`)))))

(event `AnotherRound`
  (goto _label_2))

(event `self.ReceiveTick`
  (params (DeltaSeconds :type "Float (single-precision)"))
  (bind _returnvalue (`GameplayStatics.GetActorOfClass` "/Game/Blueprints/BP_JellyBeanJar.BP_JellyBeanJar_C"))
  (`/Engine/EditorBlueprintResources/StandardMacros.IsValid` _returnvalue
    (:`Is Valid`
      (`|ExecutionSequence`
        (:`then_0`
          (if (>= (`/Game/Blueprints/BP_JellyBeanJar.Beans in Jar` _returnvalue) 5)
            (`/Engine/EditorBlueprintResources/StandardMacros.DoOnce` false
              (:`Completed`
                (bind _returnvalue_2 (`|CreateWidget` "/Game/UI/WB_YouWin.WB_YouWin_C"))
                (`UserWidget.AddToViewport` _returnvalue_2 0)
                (`GameplayStatics.SetGamePaused` true)))))
        (:`then_1`
          (if (>= (`/Game/Blueprints/BP_JellyBeanJar.Blue Beans in Jar` _returnvalue) 5)
            (`/Engine/EditorBlueprintResources/StandardMacros.DoOnce` false
              (:`Completed`
                (bind _returnvalue_3 (`|CreateWidget` "/Game/UI/WB_Player2YouWin.WB_Player2YouWin_C"))
                (`UserWidget.AddToViewport` _returnvalue_3 0)
                (`GameplayStatics.SetGamePaused` true)))))))))

(fn `UserConstructionScript`)