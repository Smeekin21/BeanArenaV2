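; BP_JellyBeanObjective2 is an interactable jelly bean objective item that the mechanic player can pick up.
; On Interact, it casts and caches player 0's character, then attaches itself to the right-hand socket.
; A successful attach adds it to the character's AlreadyHeldItems and sets HoldingItem.
; The HoldingItem guard reads the cached reference before the cast assigns it, and debug prints trace each path.
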(event `self.Interact`
  (if (`/Game/ThirdPerson/Blueprints/BP_MechanicPlayerCharacter.Holding Item?` (`self.As BP Mechanic Player Character`))
    (`KismetSystemLibrary.PrintString` "Same Item")
    (else
      (`KismetSystemLibrary.PrintString` "Hello")
      (bind _asbp_mechanic_player_character (cast `/Game/ThirdPerson/Blueprints/BP_MechanicPlayerCharacter` (`GameplayStatics.GetPlayerCharacter` 0)))
      (bind _output_get (set `self.As BP Mechanic Player Character` _asbp_mechanic_player_character))
      (bind _returnvalue (`self.K2_AttachToActor` _output_get "Hand_R_Socket" "KeepWorld" "KeepRelative" "KeepRelative"))
      (if _returnvalue
        (bind _returnvalue_2 (`KismetArrayLibrary.Array_Add` (`/Game/ThirdPerson/Blueprints/BP_MechanicPlayerCharacter.AlreadyHeldItems` _asbp_mechanic_player_character) self))
        (`KismetSystemLibrary.PrintString` (`KismetStringLibrary.Conv_IntToString` _returnvalue_2))
        (set `/Game/ThirdPerson/Blueprints/BP_MechanicPlayerCharacter.Holding Item?` true (`self.As BP Mechanic Player Character`))))))

(fn `UserConstructionScript`)