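; Explosive bullet pickup that temporarily powers up the mechanic player character who overlaps it.
; On overlap it sets the character's ExplosivePowerUp flag, hides its mesh, swaps the gun mesh to a bazooka and force-disables splitscreen.
; A 10-second delay then restores the flag and rifle mesh and destroys the actor, alongside an equally long lifespan that may expire first.
; Collision stays enabled while hidden, and a debug print remains.
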(event `self.ReceiveBeginPlay`)

(event `self.ReceiveActorBeginOverlap`
  (params (OtherActor :type "Actor Object Reference"))
  (bind _asbp_mechanic_player_character (cast `/Game/ThirdPerson/Blueprints/BP_MechanicPlayerCharacter` OtherActor))
  (set `/Game/ThirdPerson/Blueprints/BP_MechanicPlayerCharacter.ExplosivePowerUp?` true _asbp_mechanic_player_character)
  (`|ExecutionSequence`
    (:`then_0`
      (`SceneComponent.SetVisibility` (`self.StaticMesh`) false false)
      (`self.SetLifeSpan` 10.0)
      (bind _skeletalmesh (`/Game/Weapons/Rifle/BP_GunWeapon_Master.SkeletalMesh` (`/Game/ThirdPerson/Blueprints/BP_MechanicPlayerCharacter.Gun Weapon Reference` _asbp_mechanic_player_character)))
      (`SkeletalMeshComponent.SetSkeletalMeshAsset` _skeletalmesh "/Game/Models/SKM_Bazooka_by_JJ.SKM_Bazooka_by_JJ")
      (`KismetSystemLibrary.PrintString` "Bean")
      ; Splitscreen done after win
      (`GameplayStatics.SetForceDisableSplitscreen` true))
    (:`then_1`
      (`KismetSystemLibrary.Delay` 10.0)
      (set `/Game/ThirdPerson/Blueprints/BP_MechanicPlayerCharacter.ExplosivePowerUp?` false _asbp_mechanic_player_character)
      (`SkeletalMeshComponent.SetSkeletalMeshAsset` _skeletalmesh "/Game/Models/SKM_rifle.SKM_rifle")
      (`self.K2_DestroyActor`))))

(fn `UserConstructionScript`)