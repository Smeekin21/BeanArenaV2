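; BP_BulletIncreasePowerup is a pickup actor that gives the player a temporary bullet increase powerup.
; On overlap with BP_MechanicPlayerCharacter, it sets the character's BulletIncreasePowerup flag, hides its mesh and starts a ten-second lifespan.
; A parallel Delay of equal length clears the flag and destroys the actor, so the reset coincides with lifespan expiry.
; Overlap stays active while the mesh is hidden.
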(event `self.ReceiveActorBeginOverlap`
  (params (OtherActor :type "Actor Object Reference"))
  (bind _asbp_mechanic_player_character (cast `/Game/ThirdPerson/Blueprints/BP_MechanicPlayerCharacter` OtherActor))
  (set `/Game/ThirdPerson/Blueprints/BP_MechanicPlayerCharacter.Bullet Increase Powerup?` true _asbp_mechanic_player_character)
  (`|ExecutionSequence`
    (:`then_0`
      (`SceneComponent.SetVisibility` (`self.StaticMesh`) false false)
      (`self.SetLifeSpan` 10.0))
    (:`then_1`
      (`KismetSystemLibrary.Delay` 10.0)
      (set `/Game/ThirdPerson/Blueprints/BP_MechanicPlayerCharacter.Bullet Increase Powerup?` false _asbp_mechanic_player_character)
      (`self.K2_DestroyActor`))))

(fn `UserConstructionScript`
  (`parent.UserConstructionScript`))