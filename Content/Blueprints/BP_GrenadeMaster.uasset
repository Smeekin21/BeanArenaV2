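; Base grenade actor that detonates on a three-second fuse after BeginPlay while its sphere flashes an overlay material.
; Detonation runs a radial sphere trace, sending damage through BPI_Damage to only the first implementing hit via DoOnce.
; A hit without that interface triggers the Niagara impact effect and destroys the grenade.
; Sticky attachment and launch impulse logic are disconnected, leaving the overlap event empty.
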(event `self.ReceiveTick`
  (params (DeltaSeconds :type "Float (single-precision)"))
  (bind _sphere1 (`self.Sphere1`))
  (`KismetSystemLibrary.Delay` 0.2)
  (`/Engine/EditorBlueprintResources/StandardMacros.FlipFlop`
    (:`A`
      (`MeshComponent.SetOverlayMaterial` _sphere1 "/Engine/EngineMaterials/EditorBrushMaterial.EditorBrushMaterial"))
    (:`B`
      (`MeshComponent.SetOverlayMaterial` _sphere1 null))))

(event `self.ReceiveBeginPlay`
  (bind _returnvalue (`GameplayStatics.GetActorOfClass` "/Game/ThirdPerson/Blueprints/BP_MechanicPlayerCharacter.BP_MechanicPlayerCharacter_C"))
  (set `self.As BP Mechanic Player Character` _returnvalue)
  (`KismetSystemLibrary.Delay` 3.0)
  (`self.Grenade`))

(event `Grenade`
  (bind _returnvalue (`self.K2_GetActorLocation`))
  (bind _outhits (`KismetSystemLibrary.SphereTraceMulti` :`Start` _returnvalue :`End` _returnvalue :`Radius` 500.0 :`TraceChannel` "TraceTypeQuery1" :`DrawDebugType` "ForDuration"))
  (for _array_element _outhits
    (bind (_bblockinghit _binitialoverlap _time _distance _location _impactpoint _normal _impactnormal _physmat _hitactor) (`GameplayStatics.BreakHitResult` _array_element))
    (if (`KismetSystemLibrary.DoesImplementInterface` _hitactor "/Game/Blueprints/Interfaces/BPI_Damage.BPI_Damage_C")
      (`/Engine/EditorBlueprintResources/StandardMacros.DoOnce` false
        (:`Completed`
          (message `/Game/Blueprints/Interfaces/BPI_Damage.Damage` _hitactor (`self.Damage Amount`) 0.0 false null)))
      (else
        (`NiagaraFunctionLibrary.SpawnSystemAtLocation` "/Game/Mixed_Magic_VFX_Pack/VFX/Sperate_VFX/NS_Magma_Shot_Impact.NS_Magma_Shot_Impact" (`SceneComponent.K2_GetComponentLocation` (`self.Sphere1`)))
        (`self.K2_DestroyActor`)))))

(event `self.Sphere2.OnComponentBeginOverlap`
  (params (OverlappedComponent :type "PrimitiveComponent Object Reference") (OtherActor :type "Actor Object Reference") (OtherComp :type "PrimitiveComponent Object Reference") (OtherBodyIndex :type Integer) (bFromSweep :type Boolean) (SweepResult :type "HitResult Structure (by ref)"))
  ; Sentex grenade Type
)

(fn `UserConstructionScript`)