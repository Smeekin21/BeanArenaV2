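; Master gun weapon that attaches to the player's mesh socket and fires jelly bean projectiles with randomly picked materials.
; Shoot runs a looping Pew timer for automatic weapons only; each tick grows spread, expands the reticle widget and activates a Niagara effect.
; Projectiles leave the barrel socket along the follow camera's rotation plus spread and arc, decrementing ammo until firing stops.
; Recoil, hitmarker and several reticle experiments are left disconnected.
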(event `self.ReceiveBeginPlay`
  (`self.K2_AttachToComponent` (`Character.Mesh` (`self.PlayerMasterRef`)) (`self.Socket Name`) "SnapToTarget" "KeepWorld" "KeepWorld")
  (bind _asbp_third_person_game_mode (cast `/Game/ThirdPerson/Blueprints/BP_ThirdPersonGameMode` (`GameplayStatics.GetGameMode`)))
  (set `self.GameMode` _asbp_third_person_game_mode)
  (bind _returnvalue (`GameplayStatics.GetActorOfClass` "/Game/ThirdPerson/Blueprints/BP_MechanicPlayerCharacter.BP_MechanicPlayerCharacter_C"))
  (set `self.As BP Mechanic Player Character` _returnvalue)
  (bind _returnvalue_2 (`|CreateWidget` "/Game/UI/WB_Reticle.WB_Reticle_C" (`GameplayStatics.GetPlayerController` 1) null))
  (`UserWidget.AddToPlayerScreen` _returnvalue_2 0)
  (set `self.ReticleWidget` _returnvalue_2))

(event `Key|R`
  (params (Key :type "Key Structure")))

(event `Shoot`
  (bind _reticlewidget (`self.ReticleWidget`))
  (`/Engine/EditorBlueprintResources/StandardMacros.DoOnce` false :!label _label
    (:`Completed`
      (if (> (`self.CurrentAmmo`) 0)
        (set `self.Has Ammo?` true)
        (set `self.Firing?` true)
        (if (`self.Automatic?`)
          (`UserWidget.PlayAnimation` _reticlewidget (`/Game/UI/WB_Reticle.RedicalExpand` _reticlewidget) 0.0 18 "Forward" 1.0 false)
          (`self.Pew`)
          (bind _returnvalue (`KismetSystemLibrary.K2_SetTimerDelegate` (delegate `Pew`) (`self.Fire rate`) true))
          (set `self.Timer Automatic` _returnvalue))
        (else
          (set `self.Has Ammo?` false)
          (`self.Stop Firing`))))))

(event `Stop Firing`
  (bind _reticlewidget (`self.ReticleWidget`))
  (`UserWidget.PlayAnimation` _reticlewidget (`/Game/UI/WB_Reticle.RedicalExpand` _reticlewidget) 0.0 1 "Reverse" 1.0 false)
  ; Stop Firing
  (`KismetSystemLibrary.K2_ClearAndInvalidateTimerHandle` (`self.Timer Automatic`))
  (set `self.Firing?` false)
  (set `self.Spread` 0.0)
  (set `self.Delta Rotation X (Roll)` 0.0)
  (goto _label :!via `Reset`))

(event `Pew`
  (set `self.Spread` (+ (`self.Spread`) 0.1))
  (`self.ReticleExpand`)
  (`KismetSystemLibrary.PrintString` "hAPPENING")
  (bind _returnvalue (`self.Projectile Spawn Function`))
  (`ActorComponent.SetActive` (`self.NS_PowerupLight1`) true true))

(event `CountShrinkTimer`
  (set `self.StartShrink` true)
  (`self.ShrinkReticle`))

(event `Reload`
  (`KismetSystemLibrary.Delay` (`self.Reload Time`))
  (set `self.CurrentAmmo` (`self.MaxAmmo`))
  (set `self.Has Ammo?` true)
  (set `self.Firing?` true))

(event `self.ReceiveTick`
  (params (DeltaSeconds :type "Float (single-precision)"))
  ;[0.7156 0.03876 0.09953 0.5] Aimed reticle shrink
)

(event `ShrinkReticle`
  (bind _returnvalue (`GameplayStatics.GetWorldDeltaSeconds`))
  (bind _returnvalue_2 (`KismetMathLibrary.FClamp` (`self.Transform Scale Y`) 1.0))
  (bind _returnvalue_3 (`KismetMathLibrary.FClamp` (`self.Transform Scale X`) 1.0))
  ;[0 0.1099 0.9406 0.5] Reticle Shrink
  (if (`self.StartShrink`)
    (`Widget.SetRenderScale` (`/Game/UI/WB_Reticle.Redical` (`self.ReticleWidget`)) (`KismetMathLibrary.MakeVector2D` (`KismetMathLibrary.FInterpTo` _returnvalue_3 (* _returnvalue_3 1.0) _returnvalue 1.0) (`KismetMathLibrary.FInterpTo` _returnvalue_2 (* _returnvalue_2 1.0) _returnvalue 1.0)))
    (set `self.StartShrink` false)
    (`KismetSystemLibrary.K2_ClearAndInvalidateTimerHandle` (`self.ShrinkTimer`))
    (set `self.ShrinkTimerFloat` 0.0)))

(event `Hitmarker`
  ; Scott Old hitmarker
)

(event `ReticleExpand`
  (bind _returnvalue (`GameplayStatics.GetWorldDeltaSeconds`))
  (bind _redical (`/Game/UI/WB_Reticle.Redical` (`self.ReticleWidget`)))
  (bind _rendertransform (`Widget.RenderTransform` _redical))
  (bind _returnvalue_2 (`KismetMathLibrary.FInterpTo` (`.Y` (`KismetMathLibrary.BreakVector2D` (`.Scale` (break `WidgetTransform` _rendertransform)))) (* (`.Y` (`KismetMathLibrary.BreakVector2D` (`.Scale` (break `WidgetTransform` _rendertransform)))) 1.5) _returnvalue 3.0))
  (bind _returnvalue_3 (`KismetMathLibrary.FInterpTo` (`KismetMathLibrary.BreakVector2D` (`.Scale` (break `WidgetTransform` _rendertransform))) (* (`KismetMathLibrary.BreakVector2D` (`.Scale` (break `WidgetTransform` _rendertransform))) 1.5) _returnvalue 3.0))
  ;[0.9615 0.004854 0.04481 0.5] Reticle Expand
  (set `self.Transform Scale X` (`KismetMathLibrary.BreakVector2D` (`.Scale` (break `WidgetTransform` _rendertransform))))
  (set `self.Transform Scale Y` (`.Y` (`KismetMathLibrary.BreakVector2D` (`.Scale` (break `WidgetTransform` _rendertransform)))))
  (if (and (< (`self.Transform Scale X`) 1.5) (< (`self.Transform Scale Y`) 1.5))
    (set `self.Transform Scale X` _returnvalue_3)
    (set `self.Transform Scale Y` _returnvalue_2)
    (`Widget.SetRenderScale` _redical (`KismetMathLibrary.MakeVector2D` _returnvalue_3 _returnvalue_2))))

(fn `Projectile Spawn Function`
  (returns (ReturnValue :type "/Game/Blueprints/BP_JellyBean_Projectile Object Reference"))
  (bind _spread (`self.Spread`))
  (bind _playermasterref (`self.PlayerMasterRef`))
  (bind (_returnvalue_location _returnvalue_rotation) (`KismetMathLibrary.BreakTransform` (`SceneComponent.GetSocketTransform` (`self.SkeletalMesh`) "Barrel_End" "RTS_World")))
  (bind _returnvalue (`KismetMathLibrary.RandomFloatInRange` _spread (* _spread 0.0)))
  (bind (_returnvalue_roll _returnvalue_pitch _returnvalue_yaw) (`KismetMathLibrary.BreakRotator` (`KismetMathLibrary.Conv_VectorToRotator` (`SceneComponent.GetForwardVector` (`/Game/ThirdPerson/Blueprints/BP_MechanicPlayerCharacter.FollowCamera` _playermasterref)))))
  (if (`self.Can Fire?`)
    (bind _returnvalue_2 (`|SpawnActorFromClass` "/Game/Blueprints/BP_JellyBean_Projectile.BP_JellyBean_Projectile_C" (`KismetMathLibrary.MakeTransform` (+ (`KismetMathLibrary.GetForwardVector` _returnvalue_rotation) _returnvalue_location) (`KismetMathLibrary.MakeRotator` (+ _returnvalue _returnvalue_roll) (+ (+ _returnvalue _returnvalue_pitch) (`self.Arc amount`)) (+ _returnvalue _returnvalue_yaw))) "AlwaysSpawn" "MultiplyWithRoot" null null null))
    (`/Game/Blueprints/BP_JellyBean_Projectile.SetOwningPlayer` _returnvalue_2 _playermasterref)
    (`PrimitiveComponent.SetMaterial` (`/Game/Blueprints/BP_JellyBean_Projectile.Sphere` _returnvalue_2) 0 (`KismetArrayLibrary.Array_Random` (`self.Material Array`)))
    (bind _result (`/Engine/EditorBlueprintResources/StandardMacros.DecrementInt` (`self.CurrentAmmo`))
      (:`  `
        (if (<= _result 0)
          (set `self.Firing?` false)
          (set `self.Has Ammo?` false)
          ; When ammo = 0 stop firing
          (`self.Stop Firing`)
          (return _returnvalue_2)
          (else
            (return null)))))
    (else
      (`self.Stop Firing`))))

(fn `UserConstructionScript`)