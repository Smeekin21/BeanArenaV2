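; SMG weapon Blueprint that fires grenade-launcher projectiles with random materials from the barrel socket, aimed along the player camera with an added arc.
; Shoot, gated by a DoOnce, starts a looping fire-rate timer in automatic mode only; StopFiring clears it and resets the gate.
; Each shot activates a Niagara effect and calls the overridden spawn function, which spends ammo and reloads when empty.
; Recoil and parent spawn logic are disconnected.
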(event `self.Shoot`
  (`/Engine/EditorBlueprintResources/StandardMacros.DoOnce` false :!label _label
    (:`Completed`
      (if (> (`self.CurrentAmmo`) 0)
        (set `self.Has Ammo?` true)
        (set `self.Firing?` true)
        (if (`self.Automatic?`)
          (`self.Pew`)
          (bind _returnvalue (`KismetSystemLibrary.K2_SetTimerDelegate` (delegate `self.Pew`) (`self.Fire rate`) true))
          (set `self.Timer Automatic` _returnvalue))
        (else
          (set `self.Has Ammo?` false)
          (`self.Stop Firing`)
          (`self.Reload`))))))

(event `self.Stop Firing`
  (`KismetSystemLibrary.K2_ClearAndInvalidateTimerHandle` (`self.Timer Automatic`))
  (set `self.Firing?` false)
  (goto _label :!via `Reset`))

(event `self.Pew`
  (`self.Projectile Spawn Function`)
  (`ActorComponent.SetActive` (`self.NS_PowerupLight1`) true true))

(fn `Projectile Spawn Function`
  (returns (ReturnValue :type "/Game/Blueprints/BP_JellyBean_Projectile Object Reference"))
  (bind _playermasterref (`self.PlayerMasterRef`))
  (bind _returnvalue_location (`KismetMathLibrary.BreakTransform` (`SceneComponent.GetSocketTransform` (`self.SkeletalMesh`) "Barrel_End" "RTS_World")))
  (bind (_returnvalue_roll _returnvalue_pitch _returnvalue_yaw) (`KismetMathLibrary.BreakRotator` (`KismetMathLibrary.Conv_VectorToRotator` (`SceneComponent.GetForwardVector` (`/Game/ThirdPerson/Blueprints/BP_MechanicPlayerCharacter.FollowCamera` _playermasterref)))))
  (if (`self.Can Fire?`)
    (bind _returnvalue (`|SpawnActorFromClass` "/Game/Blueprints/BP_GrenadeLauncherProjectile.BP_GrenadeLauncherProjectile_C" (`KismetMathLibrary.MakeTransform` (+ (`SceneComponent.GetForwardVector` (`self.SkeletalMesh`)) _returnvalue_location) (`KismetMathLibrary.MakeRotator` _returnvalue_roll (+ _returnvalue_pitch (`self.Arc amount`)) _returnvalue_yaw)) "AlwaysSpawn" "MultiplyWithRoot" null null null))
    (`/Game/Blueprints/BP_JellyBean_Projectile.SetOwningPlayer` _returnvalue _playermasterref)
    (`PrimitiveComponent.SetMaterial` (`/Game/Blueprints/BP_JellyBean_Projectile.Sphere` _returnvalue) 0 (`KismetArrayLibrary.Array_Random` (`self.Material Array`)))
    (bind _result (`/Engine/EditorBlueprintResources/StandardMacros.DecrementInt` (`self.CurrentAmmo`))
      (:`  `
        (if (<= _result 0)
          (set `self.Firing?` false)
          (set `self.Has Ammo?` false)
          (`self.Reload`)
          (return null)
          (else
            (return null)))))
    (else
      (`self.Stop Firing`))))

(fn `UserConstructionScript`
  (`parent.UserConstructionScript`))