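; Shotgun weapon Blueprint that fires a burst of spread projectiles and reloads when empty.
; Shoot, gated by a DoOnce that StopFiring resets, fires only when Automatic is set and ammo remains.
; Each shot spawns pellets at the barrel along the randomised camera aim, setting owner and random material only on the last.
; It then applies random recoil to both player pawns and spends one ammo; Reload refills after a delay.
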(event `self.ReceiveBeginPlay`
  (`parent.ReceiveBeginPlay`))

(event `self.Shoot`
  (`/Engine/EditorBlueprintResources/StandardMacros.DoOnce` false :!label _label
    (:`Completed`
      (if (> (`self.CurrentAmmo`) 0)
        (set `self.Has Ammo?` true)
        (set `self.Firing?` true)
        (if (`self.Automatic?`)
          (`self.ShotgunPew`))
        (else
          (set `self.Has Ammo?` false)
          (`self.Stop Firing`)
          (`self.Reload`))))))

(event `self.Stop Firing`
  (`KismetSystemLibrary.K2_ClearAndInvalidateTimerHandle` (`self.Timer Automatic`))
  (set `self.Firing?` false)
  (goto _label :!via `Reset`))

(event `ShotgunPew`
  (`self.Projectile Spawn Function`))

(event `self.Reload`
  (`KismetSystemLibrary.Delay` (`self.Reload Time`))
  (set `self.CurrentAmmo` (`self.MaxAmmo`))
  (set `self.Has Ammo?` true)
  (set `self.Firing?` true)
  (set `self.Can Fire?` true)
  (`KismetSystemLibrary.PrintString` "Hello"))

(fn `Projectile Spawn Function`
  (returns (ReturnValue :type "/Game/Blueprints/BP_JellyBean_Projectile Object Reference"))
  (bind _returnvalue (`GameplayStatics.GetPlayerPawn` 1))
  (bind _returnvalue_2 (`GameplayStatics.GetPlayerPawn` 0))
  (bind _returnvalue_location (`KismetMathLibrary.BreakTransform` (`SceneComponent.GetSocketTransform` (`self.SkeletalMesh`) "Barrel_End" "RTS_World")))
  (bind (_returnvalue_roll _returnvalue_pitch _returnvalue_yaw) (`KismetMathLibrary.BreakRotator` (`KismetMathLibrary.Conv_VectorToRotator` (`SceneComponent.GetForwardVector` (`/Game/ThirdPerson/Blueprints/BP_MechanicPlayerCharacter.FollowCamera` (`self.PlayerMasterRef`))))))
  (if (`self.Can Fire?`)
    (for _ (range 8)
      (bind _returnvalue_3 (`|SpawnActorFromClass` "/Game/Blueprints/BP_ShotgunProjectile.BP_ShotgunProjectile_C" (`KismetMathLibrary.MakeTransform` (+ (`SceneComponent.GetForwardVector` (`self.SkeletalMesh`)) _returnvalue_location) (`KismetMathLibrary.MakeRotator` (+ _returnvalue_roll (`self.SpreadFunction`)) (+ (+ _returnvalue_pitch (`self.Arc amount`)) (`self.SpreadFunction`)) (+ _returnvalue_yaw (`self.SpreadFunction`))) (0.5 0.5 0.5)) "AlwaysSpawn" "MultiplyWithRoot" null null null)))
    (`/Game/Blueprints/BP_JellyBean_Projectile.SetOwningPlayer` _returnvalue_3 (`self.PlayerMasterRef`))
    (`PrimitiveComponent.SetMaterial` (`/Game/Blueprints/BP_JellyBean_Projectile.Sphere` _returnvalue_3) 0 (`KismetArrayLibrary.Array_Random` (`self.Material Array`)))
    (`Pawn.AddControllerPitchInput` _returnvalue_2 (`KismetMathLibrary.RandomFloatInRange` (`self.Recoil Amount Min Pitch`) (`self.Recoil Amount Max Pitch`)))
    (`Pawn.AddControllerYawInput` _returnvalue_2 (`KismetMathLibrary.RandomFloatInRange` (`self.Recoil Amount Min Yaw`) (`self.Recoil Amount Max Yaw`)))
    (`Pawn.AddControllerPitchInput` _returnvalue (`KismetMathLibrary.RandomFloatInRange` (`self.Recoil Amount Min Pitch`) (`self.Recoil Amount Max Pitch`)))
    (`Pawn.AddControllerYawInput` _returnvalue (`KismetMathLibrary.RandomFloatInRange` (`self.Recoil Amount Min Yaw`) (`self.Recoil Amount Max Yaw`)))
    (bind _result (`/Engine/EditorBlueprintResources/StandardMacros.DecrementInt` (`self.CurrentAmmo`))
      (:`  `
        (if (<= _result 0)
          (set `self.Can Fire?` false)
          (set `self.Has Ammo?` false)
          (`self.Reload`)
          (return null)
          (else
            (return null)))))
    (else
      (`self.Stop Firing`))))

(fn `SpreadFunction`
  (returns (ReturnValue :type "Float (double-precision)"))
  (bind _spread (`self.Spread`))
  (return (`KismetMathLibrary.RandomFloatInRange` _spread (* _spread -1.0))))

(fn `UserConstructionScript`
  (`parent.UserConstructionScript`))